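; Time trial game mode that tracks lap progress and flags when the race is complete.
; BeginPlay resets the completed lap count and builds the lap display text through a helper that formats completed over required laps.
; UpdateLap refreshes that text, then sets RaceComplete once the required count is reached, or LapCompleted otherwise.
; The lap count is not incremented here, only read after the initial reset.
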(event Custom|Update%20Lap
  (bind _laps_completed (Variables|Default|GetLaps%20Completed))
  (bind _laps_required (Variables|Default|GetLaps%20Required))
  (Variables|Default|SetLaps%20Text (Utilities|LapsasText _laps_completed _laps_required))
  (if (>= _laps_completed _laps_required)
    (Variables|Default|SetRace%20Complete? true)
    (else
      (Variables|Default|SetLapCompleted? true))))

(event EventBeginPlay
  (bind _output_get (Variables|Default|SetLaps%20Required (Variables|Default|GetLaps%20Required)))
  (bind _output_get_2 (Variables|Default|SetLaps%20Completed 0))
  (Variables|Default|SetLaps%20Text (Utilities|LapsasText _output_get_2 _output_get)))

(fn ConstructionScript)