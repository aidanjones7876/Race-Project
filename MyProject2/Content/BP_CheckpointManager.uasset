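; Checkpoint manager for the time trial mode that counts checkpoint hits and shows progress as "hit/required" text on GM_TimeTrial.
; On BeginPlay it binds to each checkpoint in its array and takes the array length as the required count.
; Once all are hit, a looping timer polls the game mode's LapCompleted flag, then clears it, restores checkpoint visibility and collision, and sets the count to a hard-coded 9, not zero.
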(event Custom|CheckPointHit
  (bind _checkpoint_count (Variables|Default|GetCheckPoint%20count))
  (bind _checkpoints_required (Variables|Default|GetCheckPoints%20Required))
  (Development|PrintString "CheckPoint Hit")
  (bind _result (Math|Integer|IncrementInt _checkpoint_count)
    (:%20%20
      (Variables|/Game/GM_TimeTrial.GM_TimeTrial_C|SetCheckPoint%20Text (Variables|Default|GetAs%20GM%20Time%20Trial) (Utilities|CheckPointstoText _result _checkpoints_required))
      (if (>= _checkpoint_count _checkpoints_required)
        (Utilities|Time|SetTimerbyEvent (delegate Custom|Reset%20CheckPoints) 1.0 true)))))

(event Custom|Reset%20CheckPoints
  (bind _as_gm_time_trial (Variables|Default|GetAs%20GM%20Time%20Trial))
  (if (Variables|/Game/GM_TimeTrial.GM_TimeTrial_C|GetLapCompleted? _as_gm_time_trial)
    (Variables|/Game/GM_TimeTrial.GM_TimeTrial_C|SetLapCompleted? _as_gm_time_trial false)
    (for _array_element (Variables|Default|GetCheckPoints)
      (Rendering|SetActorHiddenInGame _array_element false)
      (Collision|SetCollisionEnabled (Variables|/Game/BP_Checkpoint.BP_Checkpoint_C|Getcheckpoint _array_element) "QueryOnly")
      (bind _output_get (Variables|Default|SetCheckPoint%20count 9))
      (Variables|/Game/GM_TimeTrial.GM_TimeTrial_C|SetCheckPoint%20Text (Variables|Default|GetAs%20GM%20Time%20Trial) (Utilities|CheckPointstoText _output_get (Variables|Default|GetCheckPoints%20Required))))))

(event EventBeginPlay
  (bind _checkpoints (Variables|Default|GetCheckPoints))
  (bind _asgm_time_trial (Utilities|Casting|CastToGM_TimeTrial (Game|GetGameMode)))
  (Variables|Default|SetAs%20GM%20Time%20Trial _asgm_time_trial)
  (Variables|Default|SetCheckPoints%20Required (Utilities|Array|Length _checkpoints))
  (for _array_element _checkpoints
    (EventDispatchers|BindEventtoCheckpointHit _array_element (delegate Custom|CheckPointHit))
    (Variables|/Game/GM_TimeTrial.GM_TimeTrial_C|SetCheckPoint%20Text (Variables|Default|GetAs%20GM%20Time%20Trial) (Utilities|CheckPointstoText (Variables|Default|GetCheckPoint%20count) (Variables|Default|GetCheckPoints%20Required)))))

(fn ConstructionScript)